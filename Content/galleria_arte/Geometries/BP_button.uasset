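; Pressable push button actor for the art gallery, triggered with the Interact input.
; Box overlaps with the Mazzarella1 character open and close a gate, so presses register only in range.
; The Button Animation graph plays a sound and lerps the mesh between cached positions, chaining press and reversed release timelines.
; It then checks the ExternalSwitch and LightOff flags in My_GI, but no action follows.
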(event OnComponentBeginOverlap(Box)
  (params (OverlappedComponent :type Primitive%20Component%20Object%20Reference) (OtherActor :type Actor%20Object%20Reference) (OtherComp :type Primitive%20Component%20Object%20Reference) (OtherBodyIndex :type Integer) (bFromSweep :type Boolean) (SweepResult :type Hit%20Result%20Structure%20%28by%20ref%29))
  ;[1 1 1] Button interaction (push)
  (Utilities|Casting|CastToMazzarella1 OtherActor)
  (Utilities|FlowControl|Gate true) ; enters at Open
)

(event OnComponentEndOverlap(Box)
  (params (OverlappedComponent :type Primitive%20Component%20Object%20Reference) (OtherActor :type Actor%20Object%20Reference) (OtherComp :type Primitive%20Component%20Object%20Reference) (OtherBodyIndex :type Integer))
  ;[1 1 1] Button interaction (push)
  (Utilities|Casting|CastToMazzarella1 OtherActor)
  (Utilities|FlowControl|Gate true) ; enters at Close
)

(event EventBeginPlay
  (bind _button (Variables|Components|Getbutton))
  (bind _returnvalue (Transformation|GetRelativeTransform _button))
  (Variables|Default|SetOutPosition (Math|Transform|MakeTransform (.location _returnvalue) (.rotation _returnvalue) (.scale _returnvalue)))
  (Variables|Default|SetInPosition (Math|Transform|MakeTransform (- (.location _returnvalue) "0.000000,9.000000,0.000000") (.rotation _returnvalue) (.scale _returnvalue)))
  (Input|EnableInput (Game|GetPlayerController 0)))

(event Input|ActionEvents|InputActionInteract
  (params (Key :type Key%20Structure :default "None"))
  ;[1 1 1] Button interaction (push)
  (:Pressed
    (Utilities|FlowControl|Gate true
      (:Exit
        ;[1 1 1] Animation
        (|ButtonAnimation
          (:Out
            (bind _asmy_gi (Utilities|Casting|CastToMy_GI (Game|GetGameInstance)))
            (if (not (Variables|/Game/interactions/My_GI.My_GI_C|GetExternal%20Switch _asmy_gi))
              (if (Variables|/Game/interactions/My_GI.My_GI_C|GetLight%20Off _asmy_gi)
                _))))))))

(fn ConstructionScript)